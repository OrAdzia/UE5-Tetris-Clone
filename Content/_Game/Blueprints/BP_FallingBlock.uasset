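; Falling tetromino actor for a Tetris-style game.
; The construction script randomly picks one of seven shapes by offsetting its four cubes and tints their glow material with the shape's color.
; A looping timer steps it down one cell until a downward line trace from any cube hits WorldStatic.
; It then spawns colored BP_SingleBlock actors in place, spawns the next BP_FallingBlock at the top, and destroys itself.
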(event `self.ReceiveBeginPlay`
  (bind _returnvalue (`KismetSystemLibrary.K2_SetTimerDelegate` (delegate `DropBlock`) (`self.DropSpeed`) true))
  (set `self.BlockDroppingTimer` _returnvalue))

(event `DropBlock`
  (set `self.bShouldDrop?` true)
  (for _array_element (`SceneComponent.GetChildrenComponents` (`self.DefaultSceneRoot`) false)
    (bind _returnvalue (`SceneComponent.K2_GetComponentLocation` _array_element))
    (bind (_outhit _returnvalue_2) (`KismetSystemLibrary.LineTraceSingleForObjects` _returnvalue (- _returnvalue (0.0 0.0 50.0)) (`|MakeArray` "ObjectTypeQuery1" :!type "EObjectTypeQuery Enum")))
    (if _returnvalue_2
      (`/Engine/EditorBlueprintResources/StandardMacros.DoOnce` false
        (:`Completed`
          (set `self.bShouldDrop?` false)
          (`KismetSystemLibrary.K2_ClearAndInvalidateTimerHandle` (`self.BlockDroppingTimer`))))))
  (if (`self.bShouldDrop?`)
    (`self.K2_AddActorLocalOffset` (0.0 0.0 -50.0))
    (else
      (for _array_element_2 (`SceneComponent.GetChildrenComponents` (`self.DefaultSceneRoot`) false)
        (`|SpawnActorFromClass` "/Game/_Game/Blueprints/BP_SingleBlock.BP_SingleBlock_C" (`KismetMathLibrary.MakeTransform` (`SceneComponent.K2_GetComponentLocation` _array_element_2)) "Undefined" "OverrideRootScale" null (`self.BlockColor`) null))
      (`|SpawnActorFromClass` "BP_FallingBlock_C" (`KismetMathLibrary.MakeTransform` (0.0 0.0 1000.0)) "Undefined" "OverrideRootScale" null null)
      (`self.K2_DestroyActor`))))

(fn `UserConstructionScript`
  (switch `int` (`KismetMathLibrary.RandomIntegerInRange` 0 6)
    (:`0`
      ;[1 1 1] Make Line Block
      (`SceneComponent.K2_AddLocalOffset` (`self.Cube2`) (0.0 0.0 50.0) false false)
      (`SceneComponent.K2_AddLocalOffset` (`self.Cube3`) (0.0 0.0 100.0) false false)
      (`SceneComponent.K2_AddLocalOffset` (`self.Cube4`) (0.0 0.0 150.0) false false)
      (set `self.BlockColor` (struct :`R` 0.983362 :`G` 1.0 :`A` 1.0)))
    (:`1`
      ;[1 1 1] Make L Block
      (`SceneComponent.K2_AddLocalOffset` (`self.Cube2`) (0.0 0.0 50.0) false false)
      (`SceneComponent.K2_AddLocalOffset` (`self.Cube3`) (0.0 0.0 100.0) false false)
      (`SceneComponent.K2_AddLocalOffset` (`self.Cube4`) (0.0 50.0 0.0) false false)
      (set `self.BlockColor` (struct :`R` 1.0 :`B` 0.038177 :`A` 1.0)))
    (:`2`
      ;[1 1 1] Make Reverse L Block
      (`SceneComponent.K2_AddLocalOffset` (`self.Cube2`) (0.0 0.0 50.0) false false)
      (`SceneComponent.K2_AddLocalOffset` (`self.Cube3`) (0.0 0.0 100.0) false false)
      (`SceneComponent.K2_AddLocalOffset` (`self.Cube4`) (0.0 -50.0 0.0) false false)
      (set `self.BlockColor` (struct :`R` 0.989583 :`G` 0.372928 :`B` 0.009495 :`A` 1.0)))
    (:`3`
      ;[1 1 1] Make S Block
      (`SceneComponent.K2_AddLocalOffset` (`self.Cube2`) (0.0 0.0 50.0) false false)
      (`SceneComponent.K2_AddLocalOffset` (`self.Cube3`) (0.0 50.0 50.0) false false)
      (`SceneComponent.K2_AddLocalOffset` (`self.Cube4`) (0.0 50.0 100.0) false false)
      (set `self.BlockColor` (struct :`R` 1.0 :`B` 0.717084 :`A` 1.0)))
    (:`4`
      ;[1 1 1] Make Reverse S Block
      (`SceneComponent.K2_AddLocalOffset` (`self.Cube2`) (0.0 0.0 50.0) false false)
      (`SceneComponent.K2_AddLocalOffset` (`self.Cube3`) (0.0 -50.0 50.0) false false)
      (`SceneComponent.K2_AddLocalOffset` (`self.Cube4`) (0.0 -50.0 100.0) false false)
      (set `self.BlockColor` (struct :`G` 0.114498 :`B` 1.0 :`A` 1.0)))
    (:`5`
      ;[1 1 1] Make T Block
      (`SceneComponent.K2_AddLocalOffset` (`self.Cube2`) (0.0 -50.0 0.0) false false)
      (`SceneComponent.K2_AddLocalOffset` (`self.Cube3`) (0.0 50.0 0.0) false false)
      (`SceneComponent.K2_AddLocalOffset` (`self.Cube4`) (0.0 0.0 50.0) false false)
      (set `self.BlockColor` (struct :`G` 1.0 :`B` 0.912636 :`A` 1.0)))
    (:`6`
      ;[1 1 1] Make Square Block
      (`SceneComponent.K2_AddLocalOffset` (`self.Cube2`) (0.0 0.0 50.0) false false)
      (`SceneComponent.K2_AddLocalOffset` (`self.Cube3`) (0.0 50.0 0.0) false false)
      (`SceneComponent.K2_AddLocalOffset` (`self.Cube4`) (0.0 50.0 50.0) false false)
      (set `self.BlockColor` (struct :`G` 1.0 :`B` 0.028357 :`A` 1.0))))
  (`MeshComponent.SetVectorParameterValueOnMaterials` (`self.Cube1`) "GlowColor" (`KismetMathLibrary.Conv_LinearColorToVector` (`self.BlockColor`)))
  (`MeshComponent.SetVectorParameterValueOnMaterials` (`self.Cube2`) "GlowColor" (`KismetMathLibrary.Conv_LinearColorToVector` (`self.BlockColor`)))
  (`MeshComponent.SetVectorParameterValueOnMaterials` (`self.Cube3`) "GlowColor" (`KismetMathLibrary.Conv_LinearColorToVector` (`self.BlockColor`)))
  (`MeshComponent.SetVectorParameterValueOnMaterials` (`self.Cube4`) "GlowColor" (`KismetMathLibrary.Conv_LinearColorToVector` (`self.BlockColor`))))